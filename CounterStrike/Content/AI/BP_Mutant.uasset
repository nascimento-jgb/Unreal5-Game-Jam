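; Mutant AI enemy that chases and swipes at players in a two-team Terrorist versus Counter game.
; Taking damage sets the blackboard isChasing key, tallies damage per team and updates the chase flags.
; ChasePlayer runs AIMoveTo toward player controller 0 or 1, indexed by ChaseCounter; its dead-player check is disabled.
; Attack_Player sphere-traces ahead, then plays a swipe montage and damages the player hit.
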(event `self.ReceiveAnyDamage`
  (params (Damage :type "Float (single-precision)") (DamageType :type "DamageType Object Reference") (InstigatedBy :type "Controller Object Reference") (DamageCauser :type "Actor Object Reference"))
  ;[1 1 1] targetting
  (`BlackboardComponent.SetValueAsBool` (`AIBlueprintHelperLibrary.GetBlackboard` (`AIBlueprintHelperLibrary.GetAIController` self)) "isChasing" true)
  (bind _playercontroller (message `/Game/Blueprints/Interfaces/INT_PlayerController.GetPlayerControllerRef` DamageCauser))
  (if (== (`/Game/Blueprints/PC_CounterStrike.Team` _playercontroller) "/Game/Blueprints/Player/BP_Terrorist.BP_Terrorist_C")
    (bind _output_get (set `self.damage_from_terrorist` (+ Damage (`self.damage_from_terrorist`))))
    (else
      (bind _output_get_2 (set `self.damage_from_counter` (+ Damage (`self.damage_from_counter`))))))
  (if (> _output_get _output_get_2)
    (set `self.chase_terrorist` false)
    (set `self.chase_counter` true)
    (else
      (set `self.chase_counter` false)
      (set `self.chase_terrorist` true))))

(event `Attack_Player`
  (bind _returnvalue (`self.K2_GetActorLocation`))
  ;[1 1 1] attack
  (bind _outhit (`KismetSystemLibrary.SphereTraceSingleForObjects` _returnvalue (+ _returnvalue (* (`KismetMathLibrary.GetForwardVector` (`self.K2_GetActorRotation`)) 250.0)) 200.0 (`|MakeArray` "ObjectTypeQuery3" :!type "EObjectTypeQuery Enum")))
  (if true
    (bind (_bblockinghit _binitialoverlap _time _distance _location _impactpoint _normal _impactnormal _physmat _hitactor) (`GameplayStatics.BreakHitResult` _outhit))
    (cast `/Game/Blueprints/Player/BP_PlayerBase` _hitactor)
    (`self.PlayAnimMontage` "/Game/AI/Animations/Mutant_Swiping_Anim_Montage.Mutant_Swiping_Anim_Montage")
    (`GameplayStatics.ApplyDamage` _hitactor 10.0)
    (else
      (`KismetSystemLibrary.PrintString` "attack branch false"))))

(event `Chase Player`
  ;[1 1 1] chase
  (if true
    (`|AIMoveTo` self (0.0 0.0 0.0) (`GameplayStatics.GetPlayerController` (`KismetMathLibrary.Conv_BoolToInt` (`self.chase_counter`))) 200.0
      (:`then`
        (bind _gamemode (message `/Game/Blueprints/Interfaces/INT_GameMode.GetGameModeRef` (`GameplayStatics.GetGameMode` :!enabledstate Disabled) :!enabledstate Disabled))
        (bind _returnvalue (`BlueprintMapLibrary.Map_Length` (`/Game/Blueprints/GM_CounterStrike.PlayersDead` _gamemode :!enabledstate Disabled) :!enabledstate Disabled))
        (if (`KismetMathLibrary.Conv_IntToBool` _returnvalue :!enabledstate Disabled)
          (`BlackboardComponent.SetValueAsBool` (`AIBlueprintHelperLibrary.GetBlackboard` (`AIBlueprintHelperLibrary.GetAIController` self :!enabledstate Disabled) :!enabledstate Disabled) "isChasing" false :!enabledstate Disabled)
          (`KismetSystemLibrary.PrintString` "Hello" :!enabledstate Disabled)
          (else
            (`KismetSystemLibrary.PrintString` (`KismetStringLibrary.Conv_IntToString` _returnvalue :!enabledstate Disabled) :!enabledstate Disabled)))))))

(fn `UserConstructionScript`)