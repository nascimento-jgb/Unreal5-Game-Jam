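; Base weapon actor that acts as a physics-simulated world pickup, enabling physics on its Weapon component at BeginPlay.
; When a Player-tagged actor overlaps its Sphere, the server gets the player reference and scans its weapon inventory.
; A matching WeaponType sets that player's CanLootWeapon to false.
; The final CanLootWeapon check leads to no action, so looting itself is not implemented here.
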(event `self.ReceiveBeginPlay`
  (`PrimitiveComponent.SetSimulatePhysics` (`self.Weapon`) true))

(event `self.Sphere.OnComponentBeginOverlap`
  (params (OverlappedComponent :type "PrimitiveComponent Object Reference") (OtherActor :type "Actor Object Reference") (OtherComp :type "PrimitiveComponent Object Reference") (OtherBodyIndex :type Integer) (bFromSweep :type Boolean) (SweepResult :type "HitResult Structure (by ref)"))
  (if (`self.ActorHasTag` OtherActor "Player")
    (`/Engine/EditorBlueprintResources/ActorMacros.Switch Has Authority`
      (:`Authority`
        (bind _player (message `/Game/Blueprints/Interfaces/INT_PlayerBase.GetPlayerRef` OtherActor))
        (for _array_element (`/Game/Blueprints/Player/BP_PlayerBase.WeaponInventory` _player)
          (bind _asbp_weapon_base (cast `/Game/Blueprints/Weapons/BP_Weapon_Base` _array_element))
          (if (`|EnumEquality` (`/Game/Blueprints/Weapons/BP_Weapon_Base.WeaponType` _asbp_weapon_base) (`self.WeaponType`))
            (set `/Game/Blueprints/Player/BP_PlayerBase.bCanLootWeapon` false _player)))
        (if (`/Game/Blueprints/Player/BP_PlayerBase.bCanLootWeapon` _player)
          _)))))

(fn `UserConstructionScript`)