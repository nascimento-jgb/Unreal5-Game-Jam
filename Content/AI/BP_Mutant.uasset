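; BP_Mutant is an AI enemy character that chases and melee-attacks the player.
; Every tick it forces the isChasing key to true on its AI controller's Blackboard.
; Attack_Player sphere-traces forward for pawns with debug drawing and, if the hit casts to BP_PlayerBase, plays a swipe montage and applies damage immediately.
; The attack branch is hardwired to true, so the failure print never runs.
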(event `self.ReceiveTick`
  (params (DeltaSeconds :type "Float (single-precision)"))
  (`BlackboardComponent.SetValueAsBool` (`AIBlueprintHelperLibrary.GetBlackboard` (`AIBlueprintHelperLibrary.GetAIController` self)) "isChasing" true))

(event `Attack_Player`
  (bind _returnvalue (`self.K2_GetActorLocation`))
  (bind _outhit (`KismetSystemLibrary.SphereTraceSingleForObjects` :`Start` _returnvalue :`End` (+ _returnvalue (* (`KismetMathLibrary.GetForwardVector` (`self.K2_GetActorRotation`)) 250.0)) :`Radius` 200.0 :`ObjectTypes` (`|MakeArray` "ObjectTypeQuery3" :!type "EObjectTypeQuery Enum") :`DrawDebugType` "ForDuration"))
  (if true
    (bind (_bblockinghit _binitialoverlap _time _distance _location _impactpoint _normal _impactnormal _physmat _hitactor) (`GameplayStatics.BreakHitResult` _outhit))
    (cast `/Game/Blueprints/Player/BP_PlayerBase` _hitactor)
    (`self.PlayAnimMontage` "/Game/AI/Animations/Mutant_Swiping_Anim_Montage.Mutant_Swiping_Anim_Montage")
    (`GameplayStatics.ApplyDamage` _hitactor 10.0)
    (else
      (`KismetSystemLibrary.PrintString` "attack branch false"))))

(fn `UserConstructionScript`)